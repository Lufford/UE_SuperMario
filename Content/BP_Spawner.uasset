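; BP_Spawner is a trigger-box spawner that releases BigStoneEnemy actors when the side-scroller character enters it.
; On overlap by BP_2DSideScrollerCharacter, a loop spawns several enemies at one point, offset along negative world X from the spawner.
; Each loop pass also reveals a TextRender and calls Deactivate on the Box, which leaves its collision settings untouched.
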(event `self.Box.OnComponentBeginOverlap`
  (params (OverlappedComponent :type "PrimitiveComponent Object Reference") (OtherActor :type "Actor Object Reference") (OtherComp :type "PrimitiveComponent Object Reference") (OtherBodyIndex :type Integer) (bFromSweep :type Boolean) (SweepResult :type "HitResult Structure (by ref)"))
  (cast `/Game/2DSideScrollerCPP/Blueprints/BP_2DSideScrollerCharacter` OtherActor)
  (for _ (range 4)
    (`|SpawnActorFromClass` "/Game/TestingActors/BigStoneEnemy.BigStoneEnemy_C" (`KismetMathLibrary.MakeTransform` (`KismetMathLibrary.MakeVector` (- (.x (.location (`self.GetTransform` self))) 500.0) (.y (.location (`self.GetTransform` self))) (.z (.location (`self.GetTransform` self)))) (.rotation (`self.GetTransform` self)) (.scale (`self.GetTransform` self))) "Undefined" "OverrideRootScale" null null)
    (`SceneComponent.SetVisibility` (`self.TextRender`) true false)
    (`ActorComponent.Deactivate` (`self.Box`))))

(fn `UserConstructionScript`)